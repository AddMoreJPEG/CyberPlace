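; Light card actor for the stage: a plane shown as a circle, square or custom texture, positioned by latitude, longitude, distance and spin.
; SetupLight, run on construction, pushes color, exposure, opacity and feather into a dynamic material, rotates the pivot dummies, and places and scales the plane.
; Circle and Square are special-cased, growing with Feather.
; Modify functions nudge placement; SetLightCardType switches type inside an undoable editor transaction.
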(fn ConstructionScript
  (CallFunction|SetupLight)
  (Variables|Default|SetInternalLightCardIndex (Variables|Default|GetLightCard)))

(fn SetupLight
  (bind _xyoffset (Variables|Default|GetXYOffset))
  (bind _xyscale (Variables|Default|GetXYScale))
  (bind _lightcard (Variables|Default|GetLightCard))
  (bind _xyscale_2 (Variables|Default|GetXYScale))
  (bind _feather (Variables|Default|GetFeather))
  (bind _returnvalue (Math|Float|MapRangeClamped _feather 0.0 1.0 1.0 3.0))
  (Utilities|FlowControl|Sequence
    (:then_0
      ;[1 1 1] Circle and Square are Special
      (if (Utilities|Enum|Equal(Enum) (Variables|Default|GetLightCard) "NewEnumerator41")
        (Variables|Default|SetBlack 1.0)
        (Variables|Default|SetCircle true)
        (elif (Utilities|Enum|Equal(Enum) (Variables|Default|GetLightCard) "NewEnumerator42")
          (Variables|Default|SetBlack 1.0)
          (Variables|Default|SetCircle false)
          (else
            (Variables|Default|SetBlack 0.0)
            (Variables|Default|SetCircle false)))))
    (:then_1
      (bind _returnvalue_2 (Rendering|Material|CreateDynamicMaterialInstance (Variables|Default|GetPlaneCard) 0 "/Game/V1_Stage_53/SceneAdjustment/LightCards/M_PlaneMaterial.M_PlaneMaterial" "None" :!class /Script/Engine.PrimitiveComponent))
      (Variables|Default|SetMatInst _returnvalue_2)
      (Rendering|Material|SetTextureParameterValue (Variables|Default|GetMatInst) "Texture" (CallFunction|GetLightCardTexture))
      (Rendering|Material|SetScalarParameterValue (Variables|Default|GetMatInst) "XOffset" (.x _xyoffset) :!class /Script/Engine.MaterialInstanceDynamic)
      (Rendering|Material|SetScalarParameterValue (Variables|Default|GetMatInst) "YOffset" (.y _xyoffset) :!class /Script/Engine.MaterialInstanceDynamic)
      (Rendering|Material|SetScalarParameterValue (Variables|Default|GetMatInst) "Exposure" (Variables|Default|GetExposure) :!class /Script/Engine.MaterialInstanceDynamic)
      (Rendering|Material|SetVectorParameterValue (Variables|Default|GetMatInst) "Color" (Variables|Default|GetColor) :!class /Script/Engine.MaterialInstanceDynamic)
      (Rendering|Material|SetScalarParameterValue (Variables|Default|GetMatInst) "Black" (Variables|Default|GetBlack) :!class /Script/Engine.MaterialInstanceDynamic)
      (Rendering|Material|SetScalarParameterValue (Variables|Default|GetMatInst) "Opacity" (- 1.0 (Variables|Default|GetTransparency)) :!class /Script/Engine.MaterialInstanceDynamic)
      (Rendering|Material|SetScalarParameterValue (Variables|Default|GetMatInst) "Feather" (Variables|Default|GetFeather) :!class /Script/Engine.MaterialInstanceDynamic)
      (if (Variables|Default|GetCircle)
        (Rendering|Material|SetScalarParameterValue (Variables|Default|GetMatInst) "Circle" (Math|Conversions|ToFloat(Boolean) (Variables|Default|GetCircle)) :!class /Script/Engine.MaterialInstanceDynamic)))
    (:then_2
      (Transformation|SetRelativeRotation (Variables|Default|GetLatitudeDummy) (Math|Rotator|MakeRotator 0.0 (Variables|Default|GetLatitude) 0.0) false false)
      (Transformation|SetRelativeRotation (Variables|Default|GetLongitudeDummy) (Math|Rotator|MakeRotator 0.0 0.0 (Variables|Default|GetLongitude)) false false)
      (Transformation|SetRelativeLocationAndRotation (Variables|Default|GetPlaneCard) (Math|Vector|MakeVector (Variables|Default|GetDistance) 0.0 0.0) (Math|Rotator|MakeRotator (Variables|Default|GetSpin) 0.0 0.0) false false))
    (:then_3
      (if (or (Utilities|Enum|Equal(Enum) _lightcard "NewEnumerator41") (Utilities|Enum|Equal(Enum) _lightcard "NewEnumerator42"))
        (Transformation|SetRelativeScale3D (Variables|Default|GetPlaneCard) (Math|Vector|MakeVector 1.0 (* (.x _xyscale) _returnvalue) (* (.y _xyscale) _returnvalue)))
        (else
          (Transformation|SetRelativeScale3D (Variables|Default|GetPlaneCard) (Math|Vector|MakeVector 0.0 (.x _xyscale_2) (.y _xyscale_2))))))))

(fn GetLightCardTexture
  (return (Utilities|Select :Index (Variables|Default|GetLightCard) :NewEnumerator41 0 :NewEnumerator42 0 :NewEnumerator43 0)))

(fn ModifyDistance
  (params (DistanceDelta :type Float%20%28double-precision%29))
  (bind _output_get (Variables|Default|SetDistance (+ DistanceDelta (Variables|Default|GetDistance))))
  (Transformation|SetRelativeLocationAndRotation (Variables|Default|GetPlaneCard) (Math|Vector|MakeVector (Variables|Default|GetDistance) 0.0 0.0) (Math|Rotator|MakeRotator (Variables|Default|GetSpin) 0.0 0.0) false false)
  (return _output_get))

(fn ModifyLatLong
  (params (LongitudeDelta :type Float%20%28double-precision%29) (LatitudeDelta :type Float%20%28double-precision%29))
  (Utilities|FlowControl|Sequence
    (:then_0
      (bind _output_get (Variables|Default|SetLongitude (+ LongitudeDelta (Variables|Default|GetLongitude)))))
    (:then_1
      (bind _output_get_2 (Variables|Default|SetLatitude (+ LatitudeDelta (Variables|Default|GetLatitude)))))
    (:then_2
      (Transformation|SetRelativeRotation (Variables|Default|GetLatitudeDummy) (Math|Rotator|MakeRotator 0.0 (Variables|Default|GetLatitude) 0.0) false false)
      (Transformation|SetRelativeRotation (Variables|Default|GetLongitudeDummy) (Math|Rotator|MakeRotator 0.0 0.0 (Variables|Default|GetLongitude)) false false))
    (:then_3
      (return _output_get _output_get_2))))

(fn SetLightCardType
  (params (Index :type Integer))
  (Class|KismetSystemLibrary|BeginTransaction)
  (Transactions|TransactObject self)
  (bind _output_get (Variables|Default|SetLightCard (Utilities|Enum|ByteToEnumLightCardEnum (Math|Conversions|ToByte(Integer) Index))))
  (Variables|Default|SetInternalLightCardIndex _output_get)
  (CallFunction|SetupLight)
  (Class|KismetSystemLibrary|EndTransaction))