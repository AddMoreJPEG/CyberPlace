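; BP_LightCardManager spawns, lists and destroys BP_LightCard actors for scene lighting adjustment on a stage.
; New cards, of a default type or chosen by index with a display name, attach to the manager's local space and join a light card layer.
; Enumeration and destroy-all cover every light card in the scene, however it was spawned.
; A debug function prints layer contents, though its empty-layer branch never runs.
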(fn ConstructionScript)

(fn EnumerateLightCards
  ;[1 1 1] Lightcard manager can interact with any lightcard in the scene, no matter how it was spawned
  (bind _outactors (Actor|GetAllActorsOfClass "/Game/V1_Stage_53/SceneAdjustment/LightCards/BP_LightCard.BP_LightCard_C"))
  (return _outactors))

(fn CreateLightCard
  (params (LightCardIndex :type LightCardEnum%20Enum :default "NewEnumerator41"))
  (bind _returnvalue (Game|SpawnActorfromClass "/Game/V1_Stage_53/SceneAdjustment/LightCards/BP_LightCard.BP_LightCard_C" (Transformation|GetActorTransform) "AlwaysSpawn" "OverrideRootScale" self LightCardIndex 0))
  ;[1 1 1] Attach Lightcards to the owning manager so they are in its local space
  (Transformation|AttachActorToActor _returnvalue self "None" "SnapToTarget" "SnapToTarget" "SnapToTarget" true)
  (Transformation|SetActorRelativeTransform _returnvalue (Math|Transform|MakeTransform "0, 0, 0" "0, 0, 0" "1.000000,1.000000,1.000000") false false)
  (return _returnvalue))

(fn DestroyLightCard
  (params (LightCard :type BP%20Light%20Card%20Object%20Reference))
  (Actor|DestroyActor LightCard))

(fn SpawnLightCard
  (bind _lightcard (CallFunction|CreateLightCard "NewEnumerator41"))
  (Class|LayersBlueprintLibrary|AddActortoLayer _lightcard (Variables|Default|GetLightCardsLayer)))

(fn DestroyAllLightCards
  (bind _lightcards (CallFunction|EnumerateLightCards))
  (for _array_element _lightcards
    (CallFunction|DestroyLightCard _array_element)))

(fn SpewLightCardLayer
  (bind _returnvalue (Class|LayersBlueprintLibrary|GetActors (Variables|Default|GetLightCardsLayer)))
  (if (>= (Utilities|Array|Length _returnvalue) 0)
    (for _array_element _returnvalue
      (Development|PrintString (Utilities|GetDisplayName _array_element)))
    (else
      (Development|PrintString "Layer is empty"))))

(fn SpawnLightCardbyIndex
  (params (LightIndex :type Integer) (LightName :type String))
  (bind _lightcard (CallFunction|CreateLightCard (Utilities|Enum|ByteToEnumLightCardEnum (Math|Conversions|ToByte(Integer) LightIndex))))
  (Class|LayersBlueprintLibrary|AddActortoLayer _lightcard (Variables|Default|GetLightCardsLayer))
  (Variables|/Game/V1_Stage_53/SceneAdjustment/LightCards/BP_LightCard.BP_LightCard_C|SetDisplayName _lightcard LightName)
  (return _lightcard))