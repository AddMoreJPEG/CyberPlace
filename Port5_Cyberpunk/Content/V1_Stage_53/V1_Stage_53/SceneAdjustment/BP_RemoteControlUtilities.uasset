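; BP_RemoteControlUtilities is a helper Blueprint that reports the actors present in the level, presumably for Remote Control clients.
; GetAllLevelActorsInfo gathers every Actor in the world and records each one's class display name, object path and display name in an ActorInfo struct.
; It appends these to the LevelActorsInfos array and returns it; the array is not cleared within the function, and the event graph is unused.
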(event EventBeginPlay)

(event Collision|EventActorBeginOverlap
  (params (OtherActor :type Actor%20Object%20Reference)))

(event EventTick
  (params (DeltaSeconds :type Float%20%28single-precision%29)))

(fn ConstructionScript)

(fn GetAllLevelActorsInfo
  (bind _outactors (Actor|GetAllActorsOfClass "/Script/Engine.Actor"))
  (for _array_element _outactors
    (Utilities|Array|Add (LocalVariables|GetLevelActorsInfos) (Utilities|Struct|MakeActorInfo (Utilities|GetClassDisplayName (Utilities|GetClass _array_element)) (Class|KismetSystemLibrary|GetPathName _array_element) (Utilities|GetDisplayName _array_element))))
  (return (LocalVariables|GetLevelActorsInfos)))