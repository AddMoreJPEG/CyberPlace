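; BP_EventManager is a scene-adjustment Blueprint that fires named events by turning them into console commands.
; TriggerEvent looks the name up in a map and executes the matching command, such as "ce" calls into Level Blueprint events, or prints a warning if it is undefined.
; Four manual trigger functions pass preset names from an array into TriggerEvent.
; The event graph and construction script are empty.
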(event EventBeginPlay)

(event Collision|EventActorBeginOverlap
  (params (OtherActor :type Actor%20Object%20Reference)))

(event EventTick
  (params (DeltaSeconds :type Float%20%28single-precision%29)))

(fn ConstructionScript)

(fn TriggerEvent
  (params (EventName :type String))
  (if (Utilities|Map|Contains (Variables|Default|GetEventNameToConsoleCommand) EventName)
    ;[1 1 1] Execute the console command (e.g. "ce DoSomething" to run event in level blueprint)
    (LocalVariables|SetEventCommand (.Value (Utilities|Map|Find (Variables|Default|GetEventNameToConsoleCommand) EventName)))
    (Development|ExecuteConsoleCommand (LocalVariables|GetEventCommand) 0)
    (else
      (Development|PrintString (Utilities|String|Append "Event name '" EventName "' is no defined in the EventManager!")))))

(fn TriggerManualEvent0
  (CallFunction|TriggerEvent (Utilities|Array|Get(acopy) (Variables|ManualEvents|GetManualTriggerEventNames))))

(fn TriggerManualEvent1
  (CallFunction|TriggerEvent (Utilities|Array|Get(acopy) (Variables|ManualEvents|GetManualTriggerEventNames) 1)))

(fn TriggerManualEvent2
  (CallFunction|TriggerEvent (Utilities|Array|Get(acopy) (Variables|ManualEvents|GetManualTriggerEventNames) 2)))

(fn TriggerManualEvent3
  (CallFunction|TriggerEvent (Utilities|Array|Get(acopy) (Variables|ManualEvents|GetManualTriggerEventNames) 3)))